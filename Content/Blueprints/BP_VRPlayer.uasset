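; VR player pawn that sets up hand components and forwards hand-record key input.
; BeginPlay sets floor-level tracking and gives the left and right XR hands and a right-side tracker their hand side and a reference to the pawn.
; Tick caches both motion controllers' world positions.
; The right-record, left-record and delete-record actions call OnRPressed, OnLPressed and OnCPressed, whose logic lies outside these graphs.
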(event EventTick
  (params (DeltaSeconds :type Float%20%28single-precision%29))
  (Variables|Default|SetPositionLeftHand (Transformation|GetWorldLocation (Variables|Default|GetMC_Left)))
  (Variables|Default|SetPositionRightHand (Transformation|GetWorldLocation (Variables|Default|GetMC_Right))))

(event EventBeginPlay
  (Variables|/Script/GestureRecognition.XRHandComponent|SetPlayerPawn (Variables|Default|GetXR_Right) self)
  (Variables|/Script/GestureRecognition.XRHandComponent|SetPlayerPawn (Variables|Default|GetXR_Left) self)
  (Class|HeadMountedDisplayFunctionLibrary|SetTrackingOrigin "Floor")
  (bind _output_get (Variables|Default|SetHandTracker (Variables|Default|GetTracker)))
  (Variables|/Script/GestureRecognition.HandTracker|SetHandSide _output_get "Right")
  (Variables|/Script/GestureRecognition.HandTracker|SetPlayerPawn (Variables|Default|GetHandTracker) self)
  (bind _output_get_2 (Variables|Default|SetXRHandLeft (Variables|Default|GetXR_Left)))
  (Variables|/Script/GestureRecognition.XRHandComponent|SetHandSide _output_get_2 "Left")
  (bind _output_get_3 (Variables|Default|SetXRHandRight (Variables|Default|GetXR_Right)))
  (Variables|/Script/GestureRecognition.XRHandComponent|SetHandSide _output_get_3 "Right"))

(event Input|ActionEvents|InputActionRightRecord
  (params (Key :type Key%20Structure :default "None"))
  ;[0.4719 0.4719 0.4719] Press R
  (:Pressed
    (Class|VRPlayerPawn|OnRPressed)))

(event Input|ActionEvents|InputActionDeleteRecord
  (params (Key :type Key%20Structure :default "None"))
  ;[0.4719 0.4719 0.4719] Press C
  (:Pressed
    (Class|VRPlayerPawn|OnCPressed)))

(event Input|ActionEvents|InputActionLefRecord
  (params (Key :type Key%20Structure :default "None"))
  ;[0.4719 0.4719 0.4719] Press L
  (:Pressed
    (Class|VRPlayerPawn|OnLPressed)))

(fn ConstructionScript)